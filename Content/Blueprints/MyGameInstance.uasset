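; Game instance that hosts and finds multiplayer sessions through Advanced Sessions nodes.
; CreateSession stores the server name as an extra session setting, then opens ThirdPersonExampleMap as a listen server.
; FindSession searches all server types, clears the MainMenu server list and calls FillServerList to add each named result with player counts, ping, ID and session.
; Search failures and missing or wrong-type name settings only print debug messages.
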(event `CreateSession`
  (params (ServerName :type String))
  ;[1 1 1] Create Session and open TPEM as listen server
  (`CreateSessionCallbackProxyAdvanced.CreateAdvancedSession` (`|MakeArray` (`AdvancedSessionsLibrary.MakeLiteralSessionPropertyString` "ServerName" ServerName)) (`GameplayStatics.GetPlayerController` 0)
    (:`OnSuccess`
      (`GameplayStatics.OpenLevel` "ThirdPersonExampleMap" true "listen"))))

(event `FindSession`
  ;[1 1 1] Find sessions and populate server list
  (bind _results (`FindSessionsCallbackProxyAdvanced.FindSessionsAdvanced` (`GameplayStatics.GetPlayerController` 0) 0 false "AllServers")
    (:`OnSuccess`
      (`/Game/MainMenu/WBP_MainMenu.ClearServerList` (`self.MainMenu`))
      (`self.FillServerList` _results))
    (:`OnFailure`
      (`KismetSystemLibrary.PrintString` "Failed to find sessions"))))

(fn `FillServerList`
  (params (SessionResults :type "Array of BlueprintSessionResult Structure"))
  (locals (CurrentServer :type "BlueprintSessionResult Structure"))
  (bind _currentserver (`local.CurrentServer`))
  (for _array_element SessionResults
    (bind _output_get (set `local.CurrentServer` _array_element))
    (bind _extrasettings (`AdvancedSessionsLibrary.GetExtraSettings` _output_get))
    (bind _settingvalue (`AdvancedSessionsLibrary.GetSessionPropertyString` _extrasettings "ServerName")
      (:`Found`
        (`/Game/MainMenu/WBP_MainMenu.AddServer` (`self.MainMenu`) (`KismetTextLibrary.Conv_StringToText` _settingvalue) (`KismetTextLibrary.Conv_IntToText` (`FindSessionsCallbackProxy.GetMaxPlayers` _currentserver)) (`KismetTextLibrary.Conv_IntToText` (`FindSessionsCallbackProxy.GetCurrentPlayers` _currentserver)) (`KismetTextLibrary.Conv_IntToText` (`FindSessionsCallbackProxy.GetPingInMs` _currentserver)) (`KismetTextLibrary.Conv_StringToText` (`AdvancedSessionsLibrary.GetSessionID_AsString` _currentserver)) (`local.CurrentServer`)))
      (:`NotFound`
        (`KismetSystemLibrary.PrintString` "Not Found"))
      (:`WrongType`
        (`KismetSystemLibrary.PrintString` "Wrong Type")))))