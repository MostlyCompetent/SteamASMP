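; BP_ServerOnlyCube is a cube actor that damages a gameplay character when it overlaps the cube's box.
; On BeginPlay, SpawnCube assigns the cube mesh to its static mesh component.
; Box overlap casts to BP_GameplayCharacter and passes it to DamagePlayer, which sends a fixed health change through the ChangeActorHealth message with itself as instigator.
; A failed cast only prints a debug string.
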(event `self.ReceiveBeginPlay`
  (`self.SpawnCube`))

(event `SpawnCube`
  (`StaticMeshComponent.SetStaticMesh` (`self.StaticMesh`) "/Game/Geometry/Meshes/1M_Cube.1M_Cube"))

(event `self.Box.OnComponentBeginOverlap`
  (params (OverlappedComponent :type "PrimitiveComponent Object Reference") (OtherActor :type "Actor Object Reference") (OtherComp :type "PrimitiveComponent Object Reference") (OtherBodyIndex :type Integer) (bFromSweep :type Boolean) (SweepResult :type "HitResult Structure (by ref)"))
  (bind _asbp_gameplay_character (cast `/Game/Gameplay/BP_GameplayCharacter` OtherActor)
    (:`then`
      (if (== _asbp_gameplay_character OtherActor)
        (`self.DamagePlayer` _asbp_gameplay_character)))
    (:`CastFailed`
      (`KismetSystemLibrary.PrintString` "Cast failed to BP_GameplayerCharacter in BP_ServerOnlyCube" true true (struct :`G` 0.66 :`B` 1.0 :`A` 1.0) 10.0))))

(event `DamagePlayer`
  (params (Actor :type "Actor Object Reference"))
  (message `/Game/Gameplay/I_Health.ChangeActorHealth` Actor self null "NewEnumerator1" 10.0))

(fn `UserConstructionScript`)