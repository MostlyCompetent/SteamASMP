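; BP_HealthPickup is a health pickup that bobs vertically and is consumed on contact.
; Tick adds a sine-of-real-time Z offset to the static mesh each frame without delta-time scaling, so bob height depends on frame rate.
; When an actor implementing I_Health overlaps the Collision component, the pickup sends it a fixed-amount health change through that interface, then destroys itself.
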(event `self.ReceiveTick`
  (params (DeltaSeconds :type "Float (single-precision)"))
  (`SceneComponent.K2_AddWorldOffset` (`self.StaticMesh`) (`KismetMathLibrary.MakeVector` 0.0 0.0 (* (`KismetMathLibrary.Sin` (`GameplayStatics.GetRealTimeSeconds`)) 0.25)) false false))

(event `self.Collision.OnComponentBeginOverlap`
  (params (OverlappedComponent :type "PrimitiveComponent Object Reference") (OtherActor :type "Actor Object Reference") (OtherComp :type "PrimitiveComponent Object Reference") (OtherBodyIndex :type Integer) (bFromSweep :type Boolean) (SweepResult :type "HitResult Structure (by ref)"))
  (if (`KismetSystemLibrary.DoesImplementInterface` OtherActor "/Game/Gameplay/I_Health.I_Health_C")
    (message `/Game/Gameplay/I_Health.ChangeActorHealth` OtherActor self "NewEnumerator0" 50.0)
    (`self.K2_DestroyActor`)))

(fn `UserConstructionScript`)