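; Destructible enemy spawn point that periodically spawns BP_EnemyBase at its own location.
; On server BeginPlay it randomizes its spawn interval, registers with GM_Gameplay and sets its health.
; ServerStartSpawningEnemies starts a looping timer that spawns an enemy only while the game mode's enemy count is below MaxEnemiesOnce.
; On death it destroys itself and tells the game mode to update spawn points.
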(event `self.ReceiveBeginPlay`
  (bind _spawninterval (`self.SpawnInterval`))
  (`/Engine/EditorBlueprintResources/ActorMacros.Switch Has Authority`
    (:`Authority`
      (set `self.SpawnInterval` (`KismetMathLibrary.RandomFloatInRange` (* _spawninterval 0.5) (* _spawninterval 1.5)))
      (`/Game/Gameplay/GM_Gameplay.AddEnemySpawnPoint` (cast `/Game/Gameplay/GM_Gameplay` (`GameplayStatics.GetGameMode`) :!pure true) self)
      (set `/Game/Gameplay/AC_HealthComponent.Health` 100.0 (`self.AC_HealthComponent`)))))

(event `ServerStartSpawningEnemies`
  (bind _returnvalue (`KismetSystemLibrary.K2_SetTimerDelegate` (delegate `ServerSpawnNewEnemy`) (`self.SpawnInterval`) true))
  (set `self.EnemySpawnerTimerHandle` _returnvalue))

(event `ServerSpawnNewEnemy`
  (bind _asgm_gameplay (cast `/Game/Gameplay/GM_Gameplay` (`GameplayStatics.GetGameMode`) :!pure true))
  (bind _numenemies (`/Game/Gameplay/GM_Gameplay.GetNumEnemies` _asgm_gameplay))
  (if (not (>= _numenemies (`/Game/Gameplay/GM_Gameplay.MaxEnemiesOnce` _asgm_gameplay)))
    (`GameplayTask_SpawnActor.SpawnActor` (`self.GameplayTasks`) (`self.K2_GetActorLocation`) (struct) "/Game/Gameplay/Enemies/BP_EnemyBase.BP_EnemyBase_C" false null)))

(event `/Game/Gameplay/I_HealthComponent.HandleActorDeath`
  (`self.K2_DestroyActor`)
  (`/Game/Gameplay/GM_Gameplay.UpdateEnemySpawnPoint` (cast `/Game/Gameplay/GM_Gameplay` (`GameplayStatics.GetGameMode`) :!pure true)))

(fn `UserConstructionScript`)