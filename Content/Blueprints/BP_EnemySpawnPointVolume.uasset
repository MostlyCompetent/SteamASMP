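; Box volume that spawns BP_EnemySpawner forts for the gameplay stage and registers itself with GM_Gameplay.
; StartSpawningForts runs a fast looping timer until the GameMode's spawner count reaches a multiple of CurrentStage.
; Each tick box-traces between random points for WorldStatic blockers; if clear, it spawns a fort at another, independently randomized point.
; Each successfully spawned fort immediately starts spawning enemies.
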(event `self.ReceiveBeginPlay`
  (bind _asgm_gameplay (cast `/Game/Gameplay/GM_Gameplay` (`GameplayStatics.GetGameMode`)))
  (set `/Game/Gameplay/GM_Gameplay.EnemySpawnVolumeRef` self _asgm_gameplay))

(event `StartSpawningForts`
  (bind _returnvalue (`KismetSystemLibrary.K2_SetTimerDelegate` (delegate `SpawnForts`) 0.05 true))
  (set `self.SpawnTimerHandle` _returnvalue))

(event `SpawnForts`
  (`self.SpawnNewFort`)
  (bind _asgm_gameplay (cast `/Game/Gameplay/GM_Gameplay` (`GameplayStatics.GetGameMode`)))
  (if (>= (`KismetArrayLibrary.Array_Length` (`/Game/Gameplay/GM_Gameplay.EnemySpawnerRef` _asgm_gameplay)) (* (`/Game/Gameplay/GM_Gameplay.CurrentStage` _asgm_gameplay) 3))
    (`KismetSystemLibrary.K2_ClearAndInvalidateTimerHandle` (`self.SpawnTimerHandle`))))

(event `ServerSpawnNewFort`
  (params (SpawnLocation :type "Vector Structure"))
  (bind (_asynctaskproxy _spawnedactor) (`GameplayTask_SpawnActor.SpawnActor` (`self.GameplayTasks`) SpawnLocation (struct :`Yaw` 90.0) "/Game/Blueprints/BP_EnemySpawner.BP_EnemySpawner_C" false null)
    (:`Success`
      (bind _asbp_enemy_spawner (cast `/Game/Blueprints/BP_EnemySpawner` _spawnedactor))
      (`/Game/Blueprints/BP_EnemySpawner.ServerStartSpawningEnemies` _asbp_enemy_spawner))))

(fn `SpawnNewFort`
  (bind (_returnvalue_x _returnvalue_y _returnvalue_z) (`KismetMathLibrary.BreakVector` (`self.K2_GetActorLocation`)))
  (bind (_spawnvolumesize_x _spawnvolumesize_y) (`KismetMathLibrary.BreakVector2D` (`self.SpawnVolumeSize`)))
  (bind _returnvalue (/ _spawnvolumesize_y 2.0))
  (bind _returnvalue_2 (/ _spawnvolumesize_x 2.0))
  (bind _returnvalue_3 (`KismetMathLibrary.RandomFloatInRange` (- _returnvalue_y _returnvalue) (+ _returnvalue_y _returnvalue)))
  (bind _returnvalue_4 (`KismetMathLibrary.RandomFloatInRange` (- _returnvalue_x _returnvalue_2) (+ _returnvalue_x _returnvalue_2)))
  (bind _returnvalue_5 (`KismetMathLibrary.MakeVector` _returnvalue_4 _returnvalue_3 (+ _returnvalue_z 50.0)))
  (bind (_outhit _returnvalue_6) (`KismetSystemLibrary.BoxTraceSingleForObjects` :`Start` _returnvalue_5 :`End` _returnvalue_5 :`HalfSize` (1000.0 1000.0 20.0) :`ObjectTypes` (`|MakeArray` "ObjectTypeQuery1" :!type "EObjectTypeQuery Enum") :`DrawTime` 0.5))
  (if (not _returnvalue_6)
    (`self.ServerSpawnNewFort` (`KismetMathLibrary.MakeVector` _returnvalue_4 _returnvalue_3 _returnvalue_z))))

(fn `UserConstructionScript`
  (bind (_spawnvolumesize_x _spawnvolumesize_y) (`KismetMathLibrary.BreakVector2D` (`self.SpawnVolumeSize`)))
  (`BoxComponent.SetBoxExtent` (`self.SpawnVolume`) (`KismetMathLibrary.MakeVector` _spawnvolumesize_x _spawnvolumesize_y 10.0) true))