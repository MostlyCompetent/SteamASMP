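; Player controller for the main menu that shows the menu UI and enables mouse interaction.
; On BeginPlay it creates the WBP_MainMenu widget, adds it to the viewport, sets Game and UI input focused on it, and shows the cursor.
; A temporary Escape key binding quits the game.
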(event `self.ReceiveBeginPlay`
  ;[1 1 1] Create Main Menu Widget
  (bind _returnvalue (`|CreateWidget` "/Game/MainMenu/WBP_MainMenu.WBP_MainMenu_C" self))
  (set `self.MainMenu` _returnvalue)
  (bind _mainmenu (`self.MainMenu`)
    (:`then`
      (`UserWidget.AddToViewport` _mainmenu 0)
      ;[1 1 1] Set Input Mode and Show Mouse Cursor
      (`WidgetBlueprintLibrary.SetInputMode_GameAndUIEx` self (`self.MainMenu`) "DoNotLock" false)
      (set `self.bShowMouseCursor` true))
    (:`else`)))

(event `Key|Escape`
  (params (Key :type "Key Structure"))
  ;[1 0 0] TEMP
  (:`Pressed`
    (`KismetSystemLibrary.QuitGame` self "Quit")))

(fn `UserConstructionScript`)