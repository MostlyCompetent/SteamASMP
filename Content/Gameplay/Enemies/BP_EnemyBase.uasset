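; Base enemy that registers with GM_Gameplay, chases the nearest living player and attacks in a repeating loop.
; GameMode calls Initialize to start AIMoveTo, which retries on request failure and attacks when finished.
; Attack, hit-react and death flags feed the anim BP, which calls back to restart the loop or destroy the actor.
; Child actors trigger damage through I_Health, limited to one hit per attack, with authority switches handling networking.
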(event `self.ReceiveBeginPlay`
  ;[1 0.0218 0] When we start, add outrselves to the array of enemies. I also need to make sure we remove ourselves from this list after death...
  (bind _asgm_gameplay (cast `/Game/Gameplay/GM_Gameplay` (`GameplayStatics.GetGameMode`)))
  (`/Game/Gameplay/GM_Gameplay.AddEnemyToEnemiesArray` _asgm_gameplay self)
  ;[1 1 1] Set our health in our HealthComponent
  (set `/Game/Gameplay/AC_HealthComponent.Health` (`self.Health`) (`self.AC_HealthComponent`)))

(event `Initialize`
  ;[1 1 1] Called from GameMode once all players are spawned and session in progress.
  (`self.StartMovingTowardsPlayers`))

(event `StartMovingTowardsPlayers`
  ;[1 1 1] Find nearest player, move to them, then attack.
  (`AITask_MoveTo.AIMoveTo` (`AIBlueprintHelperLibrary.GetAIController` self) (0.0 0.0 0.0) (`self.GetNearestPlayer`) (`self.MoveToAcceptanceRadius`)
    (:`OnRequestFailed`
      ;;[1 1 1] If our MoveTo fails, wait then try again
      (`KismetSystemLibrary.Delay` 0.2)
      (`self.StartMovingTowardsPlayers`))
    (:`OnMoveFinished`
      (`self.AttackPlayer`))))

(event `/Game/Gameplay/I_HealthComponent.PlayHitReactAnim`
  ;[1 1 1] Called from AC_HealthComponent; set vars for anim BP
  (`/Engine/EditorBlueprintResources/ActorMacros.Switch Has Authority`
    (:`Authority`
      (set `self.bPlayHitReact` true))))

(event `AttackPlayer`
  ;[1 1 1] Attack player, set vars for anim BP
  (`/Engine/EditorBlueprintResources/ActorMacros.Switch Has Authority`
    (:`Authority`
      (set `self.bAttacking` true)
      (set `self.bCanDamage` true))
    (:`Remote`
      (`self.ServerSetAttackingAndDamage`))))

(event `ServerPlayHitReactAnim`
  ;[1 1 1] Called from AC_HealthComponent; set vars for anim BP
  (set `self.bPlayHitReact` true))

(event `ServerSetAttackingAndDamage`
  ;[1 1 1] Attack player, set vars for anim BP
  (set `self.bAttacking` true)
  (set `self.bCanDamage` true))

(event `FinishedAttacking`
  ;[1 1 1] Called from anim BP; set attacking to false and start new move->attack sequence
  (`/Engine/EditorBlueprintResources/ActorMacros.Switch Has Authority`
    (:`Authority`
      (set `self.bAttacking` false)
      (`self.StartMovingTowardsPlayers`))
    (:`Remote`
      (`self.ServerSetNotAttacking`))))

(event `ServerSetHitReact`
  ;[1 1 1] Called from anim BP; set anim vars
  (set `self.bPlayHitReact` false))

(event `ServerSetNotAttacking`
  ;[1 1 1] Called from anim BP; set attacking to false and start new move->attack sequence
  (set `self.bAttacking` false)
  (`self.StartMovingTowardsPlayers`))

(event `/Game/Gameplay/I_HealthComponent.HandleActorDeath`
  ;[1 1 1] Called from AC_HealthComponent; call Kill Enemy
  (if (not (`self.bDead`))
    (`self.KillEnemy`)))

(event `DieAfterAnimFinished`
  ;[1 1 1] Called from anim BP; wait 1 then destroy actor
  (`KismetSystemLibrary.Delay` 1.0)
  (`self.K2_DestroyActor`))

(event `KillEnemy`
  ;[1 1 1] Make sure we're setting bDead from the server
  (set `self.bDead` true))

(event `TryDamageActor`
  (params (Actor :type "Actor Object Reference"))
  ;[1 1 1] Called from child actors; if the actor returned implements the I_Health, then call ChangeActorHealth on that actor, passing in Damage (set in child actor). Right now this also means we can only deal damage to actors which implement I_Health. Eventually I'd like to change it so anything which can take damage either uses this interface OR uses the AC_HealthComponent.
  (if (and (`self.bAttacking`) (`self.bCanDamage`) (`KismetSystemLibrary.DoesImplementInterface` Actor "/Game/Gameplay/I_Health.I_Health_C"))
    (`/Engine/EditorBlueprintResources/ActorMacros.Switch Has Authority`
      (:`Authority`
        (message `/Game/Gameplay/I_Health.ChangeActorHealth` Actor (`self.GetController`) "NewEnumerator1" 25.0)
        (set `self.bCanDamage` false))
      (:`Remote`
        (`self.DamageActorAndSetNotCanDamage` Actor)))))

(event `DamageActorAndSetNotCanDamage`
  (params (Actor :type "Actor Object Reference"))
  ;[1 1 1] This is called from the server if TryDamageActor is called remotely since we need to set a var for the anim BP
  (message `/Game/Gameplay/I_Health.ChangeActorHealth` Actor (`self.GetController`) "NewEnumerator1" 25.0)
  (set `self.bCanDamage` false))

(fn `GetNearestPlayer`
  (returns (NearestPlayer1 :type "/Game/Gameplay/Characters/BP_GameplayCharacter Object Reference"))
  (locals (Distance :type "Float (double-precision)" :default 10000000000.0) (NearestPlayer :type "/Game/Gameplay/Characters/BP_GameplayCharacter Object Reference"))
  (bind _nearestplayer (`local.NearestPlayer`))
  (`/Engine/EditorBlueprintResources/ActorMacros.Switch Has Authority`
    (:`Authority`
      (bind _spawnedplayers1 (`/Game/Gameplay/GM_Gameplay.ReturnSpawnedPlayers` (cast `/Game/Gameplay/GM_Gameplay` (`GameplayStatics.GetGameMode`) :!pure true)))
      (for _array_element _spawnedplayers1
        (bind _returnvalue (`self.GetDistanceTo` _array_element self))
        (if (< _returnvalue (`local.Distance`))
          (if (not (`/Game/Gameplay/Characters/BP_GameplayCharacter.bDead` _array_element))
            (set `local.Distance` _returnvalue)
            (set `local.NearestPlayer` _array_element))))
      (`/Engine/EditorBlueprintResources/StandardMacros.IsValid` _nearestplayer
        (:`Is Valid`
          (return _nearestplayer))))))

(fn `UserConstructionScript`)