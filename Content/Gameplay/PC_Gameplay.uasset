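; Gameplay player controller that creates the HUD and pre-game screen, spawns and possesses the player's character, and registers players with GM_Gameplay.
; SpawnPlayer loads the character class from PS_Gameplay, sends it to the server, spawns at the first PlayerStart found via a SpawnActor gameplay task, then removes the pre-game screen.
; Health updates retry on a short delay, with limited attempts, until the HUD exists.
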(event `AddSelfToConnectedCharacters`
  (bind _asgm_gameplay (cast `/Game/Gameplay/GM_Gameplay` (`GameplayStatics.GetGameMode`) :!pure true))
  (bind _asgm_gameplay_2 (cast `/Game/Gameplay/GM_Gameplay` (`GameplayStatics.GetGameMode`) :!pure true))
  (if (`KismetSystemLibrary.IsServer`)
    (if (not (`/Game/Gameplay/GM_Gameplay.bHostAddedToConnectedPlayers` _asgm_gameplay_2))
      (`/Game/Gameplay/GM_Gameplay.AddConnectedPlayer` _asgm_gameplay self)
      (set `/Game/Gameplay/GM_Gameplay.bHostAddedToConnectedPlayers` true _asgm_gameplay))
    (else
      (`/Game/Gameplay/GM_Gameplay.AddConnectedPlayer` _asgm_gameplay_2 self))))

(event `UpdateHealthDisplay`
  (params (NewHealth :type "Float (double-precision)"))
  (bind _gameplayhud (`self.GameplayHUD`))
  (`/Engine/EditorBlueprintResources/StandardMacros.IsValid` _gameplayhud
    (:`Is Valid`
      (`/Game/Gameplay/WBP_GameplayHUD.UpdateHealthDisplay` _gameplayhud NewHealth)
      (goto _label :!via `Reset`))
    (:`Is Not Valid`
      (`/Engine/EditorBlueprintResources/StandardMacros.Do N` 10 :!label _label
        (:`Exit`
          (`KismetSystemLibrary.Delay` 0.1)
          (`self.UpdateHealthDisplay` NewHealth))))))

(event `self.ReceiveBeginPlay`
  (`self.CreateGameplayHUD`))

(event `CreateGameplayHUD`
  (bind _returnvalue (`|CreateWidget` "/Game/Gameplay/WBP_GameplayHUD.WBP_GameplayHUD_C" self))
  (bind _output_get (set `self.GameplayHUD` _returnvalue))
  (`UserWidget.AddToViewport` _output_get 0))

(event `CreatePreGameWidget`
  (bind _returnvalue (`|CreateWidget` "/Game/Gameplay/WBP_PreGameScreen.WBP_PreGameScreen_C" self))
  (bind _output_get (set `self.PreGameScreen` _returnvalue))
  (`UserWidget.AddToViewport` _output_get 0))

(event `RemovePreGameScreen`
  (`Widget.RemoveFromParent` (`self.PreGameScreen`)))

(event `SpawnPlayer`
  (`self.LoadPlayerInfo`)
  (bind _outactors (`GameplayStatics.GetAllActorsOfClass` "/Script/Engine.PlayerStart"))
  (bind (_returnvalue_location _returnvalue_rotation) (`KismetMathLibrary.BreakTransform` (`self.GetTransform` (`|GetArrayItem` _outactors))))
  (bind (_asynctaskproxy _spawnedactor) (`GameplayTask_SpawnActor.SpawnActor` (`self.GameplayTasks`) _returnvalue_location _returnvalue_rotation (castclass `/Game/Gameplay/BP_GameplayCharacter` (`self.CharacterClass`) :!pure true) false null)
    (:`Success`
      (bind _asbp_gameplay_character (cast `/Game/Gameplay/BP_GameplayCharacter` _spawnedactor))
      (`self.Possess` _asbp_gameplay_character)
      (`/Game/Gameplay/BP_GameplayCharacter.InitializeAfterPossess` _asbp_gameplay_character)
      (`self.RemovePreGameScreen`))
    (:`DidNotSpawn`
      (`KismetSystemLibrary.PrintString` "Did not spawn character" true true (struct :`G` 0.66 :`B` 1.0 :`A` 1.0) 10.0))))

(event `LoadPlayerInfo`
  (bind _asps_gameplay (cast `/Game/Gameplay/PS_Gameplay` (`self.PlayerState`)))
  (`/Game/Gameplay/PS_Gameplay.LoadPlayerInfo` _asps_gameplay)
  (bind _output_get (set `self.CharacterClass` (`/Game/Gameplay/PS_Gameplay.CharacterClass` _asps_gameplay)))
  (`self.ServerRecieveCharacterClass` _output_get))

(fn `GetCharacterClass`
  (returns (CharacterClass :type "/Game/Gameplay/BP_GameplayCharacter Class Reference"))
  (return (castclass `/Game/Gameplay/BP_GameplayCharacter` (`self.CharacterClass`) :!pure true)))

(fn `OnRep_CharacterClass`)

(fn `OnRep_GamemodeRef`)

(fn `OnRep_GameplayHUD`)

(fn `UserConstructionScript`)