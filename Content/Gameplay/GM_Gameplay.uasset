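; Gameplay GameMode that runs a multiplayer pre-game lobby, player spawning and enemy activation.
; PostLogin stores each PC_Gameplay in a player-info map (health, Steam name, readiness) and pushes the list to every client's widget.
; Once all players are ready, TrySpawnPlayers spawns them, sets the session InProgress and starts registered enemies and spawners.
; During play, list updates trigger SpawnNewPlayer, which recursively spawns pawnless players with reset health after short delays.
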(event `self.ReceiveBeginPlay`
  (bind _outactors (`GameplayStatics.GetAllActorsOfClass` "/Script/Engine.PlayerStart"))
  (set `self.PlayerSpawnPoints` _outactors))

(event `self.K2_PostLogin`
  (params (NewPlayer :type "PlayerController Object Reference"))
  (bind _aspc_gameplay (cast `/Game/Gameplay/PC_Gameplay` NewPlayer))
  (`/Game/Gameplay/PC_Gameplay.CreatePreGameWidget` _aspc_gameplay)
  (`BlueprintMapLibrary.Map_Add` (`self.ConnectedPlayers`) _aspc_gameplay (make `/Game/Gameplay/S_PlayerInfo` :`Health` 100.0 :`Character` "/Game/Gameplay/Characters/BP_GameplayCharacter.BP_GameplayCharacter_C"))
  (`self.UpdateConnectedPlayersInfo` _aspc_gameplay)
  (if (`self.HasMatchStarted`)
    _))

(event `UpdateConnectedPlayersInfo`
  (params (NewPlayer :type "PC_Gameplay Object Reference") (ReadyToPlay :type Boolean))
  (bind _aspc_gameplay (cast `/Game/Gameplay/PC_Gameplay` NewPlayer :!pure true))
  (if (`KismetStringLibrary.IsEmpty` (`AdvancedSessionsLibrary.GetPlayerName` NewPlayer))
    (`KismetSystemLibrary.PrintString` "Could not get Steam Username" true true (struct :`R` 1.0 :`B` 0.009271 :`A` 1.0) 10.0)
    (else
      (bind _structout (setmembers `/Game/Gameplay/S_PlayerInfo` :`StructRef` (`BlueprintMapLibrary.Map_Find` (`self.ConnectedPlayers`) _aspc_gameplay) :`SteamUsername` (`KismetTextLibrary.Conv_StringToText` (`AdvancedSessionsLibrary.GetPlayerName` _aspc_gameplay)) :`ReadyToPlay` ReadyToPlay))
      (`BlueprintMapLibrary.Map_Add` (`self.ConnectedPlayers`) _aspc_gameplay _structout)
      (`self.UpdatePlayerList`))))

(event `SpawnNewPlayer`
  (bind _keys (`BlueprintMapLibrary.Map_Keys` (`self.ConnectedPlayers`)))
  (for _array_element _keys
    (`/Engine/EditorBlueprintResources/StandardMacros.IsValid` (`Controller.K2_GetPawn` _array_element)
      (:`Is Not Valid`
        ;[1 1 1] In case we're respawning, make sure to reset health
        (bind _structout (setmembers `/Game/Gameplay/S_PlayerInfo` :`StructRef` (`BlueprintMapLibrary.Map_Find` (`self.ConnectedPlayers`) _array_element) :`Health` (`self.DefaultHealth`)))
        (`BlueprintMapLibrary.Map_Add` (`self.ConnectedPlayers`) _array_element _structout)
        (`/Game/Gameplay/PC_Gameplay.SpawnPlayer` _array_element)
        (`KismetSystemLibrary.Delay` 0.2)
        (`self.SpawnNewPlayer`)))))

(event `UpdatePlayerList`
  (`KismetArrayLibrary.Array_Clear` (`self.PlayerSteamNameArray`))
  (`KismetArrayLibrary.Array_Clear` (`self.PlayersReady`))
  (bind _keys (`BlueprintMapLibrary.Map_Keys` (`self.ConnectedPlayers`)))
  (for _array_element _keys
    (bind ((`SteamUsername_9_2617255D419E78A67D40EF9323DDC161` _steamusername) (`ReadyToPlay_11_81F7FBD54445C4B6D6A3DBA67B3657D2` _readytoplay)) (break `/Game/Gameplay/S_PlayerInfo` (`BlueprintMapLibrary.Map_Find` (`self.ConnectedPlayers`) _array_element)))
    (`KismetArrayLibrary.Array_Add` (`self.PlayerSteamNameArray`) _steamusername)
    (`KismetArrayLibrary.Array_Add` (`self.PlayersReady`) _readytoplay))
  (bind _keys_2 (`BlueprintMapLibrary.Map_Keys` (`self.ConnectedPlayers`)))
  (for _array_element_2 _keys_2
    (`/Game/Gameplay/PC_Gameplay.UpdatePlayerListWidget` _array_element_2 (`self.PlayerSteamNameArray`) (`self.PlayersReady`)))
  (switch `/Game/Gameplay/ESessionState` (`self.SessionState`)
    (:`NewEnumerator1`
      (`self.SpawnNewPlayer`))))

(event `TrySpawnPlayers`
  (if (`self.CheckIfAllPlayersReady`)
    (`self.SpawnAllPlayers`)
    (else
      (`KismetSystemLibrary.PrintString` "Not all players ready"))))

(event `SpawnAllPlayers`
  (bind _keys (`BlueprintMapLibrary.Map_Keys` (`self.ConnectedPlayers`)))
  (for _array_element _keys
    (`/Game/Gameplay/PC_Gameplay.SpawnPlayer` _array_element))
  (set `self.SessionState` "NewEnumerator1")
  (`self.ActivateEnemies`)
  (`self.ActivateSpawnPoints`))

(fn `ActivateEnemies`
  (for _array_element (`self.Enemies`)
    (`/Game/Gameplay/Enemies/BP_EnemyBase.Initialize` _array_element)))

(fn `ActivateSpawnPoints`
  (for _array_element (`self.EnemySpawnerRef`)
    (`/Game/Blueprints/BP_EnemySpawner.ServerStartSpawningEnemies` _array_element)))

(fn `AddConnectedPlayer`
  (params (NewPlayer :type "/Game/Gameplay/PC_Gameplay Object Reference"))
  (`BlueprintMapLibrary.Map_Add` (`self.ConnectedPlayers`) NewPlayer (make `/Game/Gameplay/S_PlayerInfo` 100.0)))

(fn `AddEnemySpawnPoint`
  (params (SpawnPoint :type "/Game/Blueprints/BP_EnemySpawner Object Reference (by ref)"))
  (`KismetArrayLibrary.Array_Add` (`self.EnemySpawnerRef`) SpawnPoint))

(fn `AddEnemyToEnemiesArray`
  (params (Enemy :type "/Game/Gameplay/Enemies/BP_EnemyBase Object Reference"))
  (`KismetArrayLibrary.Array_Add` (`self.Enemies`) Enemy))

(fn `CheckIfAllPlayersReady`
  (returns (Ready :type Boolean))
  (locals (bAllPlayersReady :type Boolean))
  (set `local.bAllPlayersReady` false)
  (bind _keys (`BlueprintMapLibrary.Map_Keys` (`self.ConnectedPlayers`)))
  (for _array_element _keys
    (if (`/Game/Gameplay/PC_Gameplay.bReadyToSpawn` _array_element)
      (set `local.bAllPlayersReady` true)
      (else
        (set `local.bAllPlayersReady` false)
        (break))))
  (return (`local.bAllPlayersReady`)))

(fn `GetConnectedPlayersArray`
  (returns (ConnectedPlayers :type "Array of /Game/Gameplay/PC_Gameplay Object Reference"))
  (bind _keys (`BlueprintMapLibrary.Map_Keys` (`self.ConnectedPlayers`)))
  (return _keys))

(fn `GetNumEnemies`
  (returns (NumEnemies :type Integer))
  (return (`KismetArrayLibrary.Array_Length` (`self.Enemies`))))

(fn `OnRep_Damage`)

(fn `ReturnPlayerHealth`
  (params (Player :type "/Game/Gameplay/PC_Gameplay Object Reference"))
  (returns (Health :type "Float (double-precision)"))
  (return (`.Health_3_0860DC864BD372BFDF3C679CB5F8147A` (break `/Game/Gameplay/S_PlayerInfo` (`BlueprintMapLibrary.Map_Find` (`self.ConnectedPlayers`) Player)))))

(fn `ReturnSpawnedPlayers`
  (returns (SpawnedPlayers1 :type "Array of /Game/Gameplay/Characters/BP_GameplayCharacter Object Reference"))
  (locals (SpawnedPlayers :type "Array of /Game/Gameplay/Characters/BP_GameplayCharacter Object Reference"))
  (bind _keys (`BlueprintMapLibrary.Map_Keys` (`self.ConnectedPlayers`)))
  (for _array_element _keys
    (bind _returnvalue (`Controller.K2_GetPawn` _array_element))
    (`/Engine/EditorBlueprintResources/StandardMacros.IsValid` _returnvalue
      (:`Is Valid`
        (`KismetArrayLibrary.Array_Add` (`local.SpawnedPlayers`) (cast `/Game/Gameplay/Characters/BP_GameplayCharacter` _returnvalue :!pure true)))))
  (return (`local.SpawnedPlayers`)))

(fn `SetPlayerHealth`
  (params (Player :type "/Game/Gameplay/PC_Gameplay Object Reference") (NewHealth :type "Float (double-precision)"))
  (bind _structout (setmembers `/Game/Gameplay/S_PlayerInfo` :`StructRef` (`BlueprintMapLibrary.Map_Find` (`self.ConnectedPlayers`) Player) :`Health` NewHealth))
  (`BlueprintMapLibrary.Map_Add` (`self.ConnectedPlayers`) Player _structout))

(fn `Update Enemies Array`
  (locals (NewEnemies :type "Array of /Game/Gameplay/Enemies/BP_EnemyBase Object Reference"))
  (for _array_element (`self.Enemies`)
    (`/Engine/EditorBlueprintResources/StandardMacros.IsValid` _array_element
      (:`Is Valid`
        (`KismetArrayLibrary.Array_Add` (`local.NewEnemies`) _array_element))))
  (set `self.Enemies` (`local.NewEnemies`)))

(fn `UpdateEnemySpawnPoint`
  (locals (NewSpawnPoints :type "Array of /Game/Blueprints/BP_EnemySpawner Object Reference"))
  (for _array_element (`self.EnemySpawnerRef`)
    (`/Engine/EditorBlueprintResources/StandardMacros.IsValid` _array_element
      (:`Is Valid`
        (`KismetArrayLibrary.Array_Add` (`local.NewSpawnPoints`) _array_element))))
  (set `self.EnemySpawnerRef` (`local.NewSpawnPoints`)))

(fn `UserConstructionScript`)