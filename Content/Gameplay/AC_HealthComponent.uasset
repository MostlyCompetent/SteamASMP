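; Actor component that tracks an actor's Health and reports hits and death to its owner.
; ChangeActorHealth adds or subtracts an amount by change type, without clamping, then sends the owner a hit-react message, even for additions.
; At zero or below, it sends a death message through I_HealthComponent, or prints a warning if the owner lacks that interface.
; Health has an OnRep function, which is empty.
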(event `ChangeActorHealth`
  (params (Instigator :type "Actor Object Reference") (ChangeType :type "/Game/Gameplay/EChangeHealthType Enum" :default "NewEnumerator0") (Amount :type "Float (double-precision)"))
  (set `self.Health` (+ (`self.Health`) (* Amount (select `/Game/Gameplay/EChangeHealthType` ChangeType :`NewEnumerator0` 1.0 :`NewEnumerator1` -1.0 :!type "Float (single-precision)"))))
  (message `/Game/Gameplay/I_HealthComponent.PlayHitReactAnim` (`self.GetOwner`))
  (if (<= (`self.Health`) 0.0)
    (if (`KismetSystemLibrary.DoesImplementInterface` (`self.GetOwner`) "/Game/Gameplay/I_HealthComponent.I_HealthComponent_C")
      (message `/Game/Gameplay/I_HealthComponent.HandleActorDeath` (`self.GetOwner`))
      (else
        (`KismetSystemLibrary.PrintString` (`KismetStringLibrary.Concat_StrStr` (`KismetSystemLibrary.GetDisplayName` (`self.GetOwner`)) " uses AC_HealthCompoentn, but does not impliment I_HealthComponent"))))))

(fn `OnRep_Health`)