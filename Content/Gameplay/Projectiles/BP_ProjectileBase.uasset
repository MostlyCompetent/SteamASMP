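; BP_ProjectileBase is a projectile base class that changes the health of what it hits, either directly or within an explosion radius.
; On overlap, only the server acts: it ignores its owner, instigator and other projectiles, then destroys itself and applies the change, crediting the owner cached at BeginPlay.
; Targets receive it through AC_HealthComponent, falling back to an interface message.
; Replicated destruction spawns the hit VFX without RPCs.
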(event `self.ReceiveBeginPlay`
  ;[1 1 1] This is set because it doesn't properly get called at the end
  (set `self.MyOwner` (`self.GetOwner`)))

(event `self.Collision.OnComponentBeginOverlap`
  (params (OverlappedComponent :type "PrimitiveComponent Object Reference") (OtherActor :type "Actor Object Reference") (OtherComp :type "PrimitiveComponent Object Reference") (OtherBodyIndex :type Integer) (bFromSweep :type Boolean) (SweepResult :type "HitResult Structure (by ref)"))
  (bind _hitactor (`self.HitActor`))
  (bind _hitactor_2 (`self.HitActor`))
  (bind _returnvalue (`GameplayStatics.GetObjectClass` (`self.HitActor`)))
  (bind _returnvalue_2 (`self.GetComponentByClass` _hitactor_2 "/Game/Gameplay/AC_HealthComponent.AC_HealthComponent_C"))
  (set `self.HitActor` OtherActor)
  (`/Engine/EditorBlueprintResources/ActorMacros.Switch Has Authority`
    (:`Authority`
      (if (not (or (== _hitactor (`self.GetInstigator`)) (== _hitactor (`self.GetOwner`)) (== _hitactor self) (== _returnvalue "BP_ProjectileBase_C") (`KismetMathLibrary.ClassIsChildOf` _returnvalue "BP_ProjectileBase_C")))
        (`self.K2_DestroyActor`)
        (if (`self.bRadialDamage`)
          (bind (_outactors _returnvalue_3) (`KismetSystemLibrary.SphereOverlapActors` (`self.K2_GetActorLocation`) (`self.ExplosionRadius`) (`|MakeArray` "ObjectTypeQuery3" "ObjectTypeQuery2" :!type "EObjectTypeQuery Enum")))
          (if _returnvalue_3
            ;[1 1 1] If the actor has a health component, use that, otherwise, use the interface. Simple actors (doors, boxes, etc.) will use the component while more complex ones will use the interface.
            (for _array_element _outactors
              (bind _returnvalue_4 (`self.GetComponentByClass` _array_element "/Game/Gameplay/AC_HealthComponent.AC_HealthComponent_C"))
              (`/Engine/EditorBlueprintResources/StandardMacros.IsValid` _returnvalue_4
                (:`Is Valid`
                  (`/Game/Gameplay/AC_HealthComponent.ChangeActorHealth` _returnvalue_4 (`self.MyOwner`) "NewEnumerator1" (`self.DamageAmount`)))
                (:`Is Not Valid`
                  (message `/Game/Gameplay/I_Health.ChangeActorHealth` _array_element (`self.MyOwner`) "NewEnumerator1" (`self.DamageAmount`))))))
          (else
            (`/Engine/EditorBlueprintResources/StandardMacros.IsValid` _returnvalue_2
              (:`Is Valid`
                (`/Game/Gameplay/AC_HealthComponent.ChangeActorHealth` _returnvalue_2 (`self.MyOwner`) "NewEnumerator1" (`self.DamageAmount`)))
              (:`Is Not Valid`
                (message `/Game/Gameplay/I_Health.ChangeActorHealth` _hitactor_2 (`self.MyOwner`) "NewEnumerator1" (`self.DamageAmount`))))))))))

(event `self.ReceiveDestroyed`
  (bind _returnvalue_location (`KismetMathLibrary.BreakTransform` (`self.GetTransform`)))
  ;[1 1 1] Destruction is replicated, so we don't need any RPCs called here
  (`/Engine/EditorBlueprintResources/StandardMacros.IsValid` (`self.HitVFX`)
    (:`Is Valid`
      (`GameplayStatics.SpawnEmitterAtLocation` (`self.HitVFX`) _returnvalue_location))))

(fn `UserConstructionScript`)