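; Paladin character Blueprint that handles melee sword hits against actors with a health component.
; SwordCollision overlaps apply a fixed health change through AC_HealthComponent, passing the instigator, while CanDamage is true.
; A hit then clears CanDamage, which nothing in these graphs re-enables, limiting hits until it is reset.
; ServerPlaySwordHitEffect spawns an explosion emitter at the sweep result's hit actor, if valid.
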(event `self.SwordCollision.OnComponentBeginOverlap`
  (params (OverlappedComponent :type "PrimitiveComponent Object Reference") (OtherActor :type "Actor Object Reference") (OtherComp :type "PrimitiveComponent Object Reference") (OtherBodyIndex :type Integer) (bFromSweep :type Boolean) (SweepResult :type "HitResult Structure (by ref)"))
  (bind _returnvalue (`self.GetComponentByClass` OtherActor "/Game/Gameplay/AC_HealthComponent.AC_HealthComponent_C"))
  (if (`self.bCanDamage`)
    (`/Engine/EditorBlueprintResources/StandardMacros.IsValid` _returnvalue
      (:`Is Valid`
        (`/Game/Gameplay/AC_HealthComponent.ChangeActorHealth` _returnvalue (`self.GetInstigator`) "NewEnumerator1" 20.0)
        (`self.ServerPlaySwordHitEffect` SweepResult)
        (set `self.bCanDamage` false)))))

(event `ServerPlaySwordHitEffect`
  (params (HitResult :type "HitResult Structure"))
  (bind (_bblockinghit _binitialoverlap _time _distance _location _impactpoint _normal _impactnormal _physmat _hitactor) (`GameplayStatics.BreakHitResult` HitResult))
  (`/Engine/EditorBlueprintResources/StandardMacros.IsValid` _hitactor
    (:`Is Valid`
      (`GameplayStatics.SpawnEmitterAtLocation` "/Game/ParticleEffects/P_Explosion.P_Explosion" (`self.K2_GetActorLocation` _hitactor)))))

(fn `UserConstructionScript`
  (`parent.UserConstructionScript`))