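; BP_Archer is a playable archer character with a ranged primary attack and a collision-based secondary attack.
; ServerStartPrimaryAttack spawns a BP_ArcherArrow at the arrow spawn point, aimed along the follow camera, passing damage, owning controller and instigator.
; SecondaryAttackCollision overlaps apply damage through the other actor's AC_HealthComponent, then clear CanDamage so only one hit lands until the flag is set again.
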(event `self.ServerStartPrimaryAttack`
  (`|SpawnActorFromClass` "/Game/Gameplay/Projectiles/BP_ArcherArrow.BP_ArcherArrow_C" (`KismetMathLibrary.MakeTransform` (`SceneComponent.K2_GetComponentLocation` (`self.ArrowSpawnPoint`)) (`SceneComponent.K2_GetComponentRotation` (`self.FollowCamera`))) "AlwaysSpawn" "OverrideRootScale" (`self.GetController`) (`self.PrimaryAttackDamage`) self))

(event `self.SecondaryAttackCollision.OnComponentBeginOverlap`
  (params (OverlappedComponent :type "PrimitiveComponent Object Reference") (OtherActor :type "Actor Object Reference") (OtherComp :type "PrimitiveComponent Object Reference") (OtherBodyIndex :type Integer) (bFromSweep :type Boolean) (SweepResult :type "HitResult Structure (by ref)"))
  (bind _returnvalue (`self.GetComponentByClass` OtherActor "/Game/Gameplay/AC_HealthComponent.AC_HealthComponent_C"))
  (if (`self.bCanDamage`)
    (`/Engine/EditorBlueprintResources/StandardMacros.IsValid` _returnvalue
      (:`Is Valid`
        (`/Game/Gameplay/AC_HealthComponent.ChangeActorHealth` _returnvalue (`self.GetInstigator`) "NewEnumerator1" (`self.SecondaryAttackDamage`))
        (set `self.bCanDamage` false)))))

(fn `UserConstructionScript`
  (`parent.UserConstructionScript`))