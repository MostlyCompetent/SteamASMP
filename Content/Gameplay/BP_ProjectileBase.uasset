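; Base projectile actor that explodes on impact and deals radial damage to nearby actors.
; On authority, a hit on anything but itself, its owner or its instigator spawns an explosion emitter, destroys the projectile and sphere-overlaps Pawn and WorldDynamic objects.
; Damage goes through AC_HealthComponent on simple actors, falling back to an interface message for complex ones.
; The owner is cached at BeginPlay to serve as damage instigator.
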(event `self.ReceiveBeginPlay`
  ;[1 1 1] This is set because it doesn't properly get called at the end
  (set `self.MyOwner` (`self.GetOwner`)))

(event `self.Collision.OnComponentHit`
  (params (HitComponent :type "PrimitiveComponent Object Reference") (OtherActor :type "Actor Object Reference") (OtherComp :type "PrimitiveComponent Object Reference") (NormalImpulse :type "Vector Structure") (Hit :type "HitResult Structure (by ref)"))
  (`/Engine/EditorBlueprintResources/ActorMacros.Switch Has Authority`
    (:`Authority`
      (set `self.HitLocation` (`.Location` (`GameplayStatics.BreakHitResult` Hit)))
      (if (not (or (== OtherActor (`self.GetInstigator`)) (== OtherActor (`self.GetOwner`)) (== OtherActor self)))
        (`GameplayStatics.SpawnEmitterAtLocation` "/Game/StarterContent/Particles/P_Explosion.P_Explosion" (`self.HitLocation`))
        (`self.K2_DestroyActor`)
        (bind (_outactors _returnvalue) (`KismetSystemLibrary.SphereOverlapActors` (`self.K2_GetActorLocation`) (`self.ExplosionRadius`) (`|MakeArray` "ObjectTypeQuery3" "ObjectTypeQuery2" :!type "EObjectTypeQuery Enum")))
        (if _returnvalue
          ;[1 1 1] If the actor has a health component, use that, otherwise, use the interface. Simple actors (doors, boxes, etc.) will use the component while more complex ones will use the interface.
          (for _array_element _outactors
            (bind _returnvalue_2 (`self.GetComponentByClass` _array_element "/Game/Gameplay/AC_HealthComponent.AC_HealthComponent_C"))
            (`/Engine/EditorBlueprintResources/StandardMacros.IsValid` _returnvalue_2
              (:`Is Valid`
                (`/Game/Gameplay/AC_HealthComponent.ChangeActorHealth` _returnvalue_2 (`self.MyOwner`) "NewEnumerator1" (`self.DamageAmount`)))
              (:`Is Not Valid`
                (message `/Game/Gameplay/I_Health.ChangeActorHealth` _array_element (`self.MyOwner`) "NewEnumerator1" (`self.DamageAmount`))))))))))

(fn `UserConstructionScript`)